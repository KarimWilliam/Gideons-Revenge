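; A treasure chest Blueprint that only pawns holding a required keycard gameplay tag can open or close.
; Interact checks the tag on the instigator's SActionComponent, printing a red debug message when it is missing.
; A FlipFlop alternately plays and reverses a timeline that pitches the lid mesh, and a particle burst activates once the lid finishes opening.
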(event EventBeginPlay)

(event Collision|EventActorBeginOverlap
  (params (OtherActor :type Actor%20Object%20Reference)))

(event EventTick
  (params (DeltaSeconds :type Float%20%28single-precision%29)))

(event EventInteract
  (params (InstigatorPawn :type Pawn%20Object%20Reference))
  ;[1 1 1] Checksi f player has required keycard (gameplay tag)
  (if (GameplayTags|HasTag (Variables|/Script/ActionRoguelike.SActionComponent|GetActiveGamePlayTags (Actor|GetComponentbyClass InstigatorPawn "/Script/ActionRoguelike.SActionComponent")) (Variables|Default|GetRequiredKeyCsrd) true)
    (bind _isa (Utilities|FlowControl|FlipFlop)
      (:A
        (bind _pitch (Timeline|AnimateLid Play)
          (:Update
            (Transformation|SetRelativeRotation (Variables|Default|GetLidMesh) (Math|Rotator|MakeRotator _pitch 0.0 0.0) false false))
          (:Finished
            (if _isa
              (Components|Activation|Activate (Variables|Default|GetP_Hud_Fire_Dmg_Burst) false)))))
      (:B
        (Timeline|AnimateLid Reverse)))
    (else
      (Development|PrintString (Utilities|String|Append "Missing Tag : " (GameplayTags|GetDebugStringfromGameplayTag (Variables|Default|GetRequiredKeyCsrd))) true true "(R=1.000000,G=0.049777,B=0.000000,A=1.000000)"))))

(fn ConstructionScript)